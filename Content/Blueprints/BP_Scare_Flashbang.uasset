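; BP_Scare_Flashbang is a scare actor that flies at the player's drone and then destroys itself.
; It starts with its mesh hidden and reveals it when the referenced Objective actor is destroyed.
; Every tick it rotates to face the drone, which it gets through the game instance.
; DoFlashBange plays a timeline that lerps it from its current location toward the drone's FlashPoint, destroying it on finish.
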(event Custom|visable
  (params (DestroyedActor :type Actor%20Object%20Reference))
  (Rendering|SetVisibility (Variables|Default|GetStaticMeshComponent) true false))

(event EventBeginPlay
  (bind _ascc_game_instance (Utilities|Casting|CastToCC_GameInstance (Game|GetGameInstance)))
  (Variables|Default|SetGameInstance _ascc_game_instance)
  (Game|BindEventtoOnDestroyed (Variables|Default|Getobjective) (delegate Custom|visable))
  (Rendering|SetVisibility (Variables|Default|GetStaticMeshComponent) false false))

(event EventTick
  (params (DeltaSeconds :type Float%20%28single-precision%29))
  (Transformation|SetActorRotation (Math|Rotator|FindLookatRotation (Transformation|GetActorLocation) (Transformation|GetActorLocation (Variables|/Script/HorrorGame.CC_GameInstance|GetDroneRef (Variables|Default|GetGameInstance))))))

(event EventDoFlashBange
  (bind _newtrack_0 (Timeline|Timeline Play)
    (:Update
      (Transformation|SetActorLocation (Math|Vector|Lerp(Vector) (Transformation|GetActorLocation) (Transformation|GetWorldLocation (Variables|/Script/HorrorGame.CC_Drone|GetFlashPoint (Variables|/Script/HorrorGame.CC_GameInstance|GetDroneRef (Variables|Default|GetGameInstance)))) _newtrack_0) false false))
    (:Finished
      (Actor|DestroyActor))))

(fn ConstructionScript)